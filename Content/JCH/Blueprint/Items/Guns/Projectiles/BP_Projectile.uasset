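; BP_Projectile is a gun projectile that launches at its Velocity variable on BeginPlay and deals fixed point damage on hit.
; The damage passes the owner's location as the hit direction.
; It then has the owning BP_Gun spawn impact FX using the physical material of the hit component's first material, or Metal if none.
; It destroys itself afterwards, only if the BP_Gun cast succeeds.
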(event `self.ReceiveBeginPlay`
  (set `MovementComponent.Velocity` (`self.Velocity`) (`self.Movement`)))

(event `self.ReceiveHit`
  (params (MyComp :type "PrimitiveComponent Object Reference") (Other :type "Actor Object Reference") (OtherComp :type "PrimitiveComponent Object Reference") (bSelfMoved :type Boolean) (HitLocation :type "Vector Structure") (HitNormal :type "Vector Structure") (NormalImpulse :type "Vector Structure") (Hit :type "HitResult Structure (by ref)"))
  (bind _returnvalue (`self.GetOwner`))
  (bind _returnvalue_2 (`PrimitiveComponent.GetMaterial` OtherComp 0))
  (`GameplayStatics.ApplyPointDamage` Other 15.0 (`self.K2_GetActorLocation` _returnvalue) Hit (`self.GetInstigatorController`) _returnvalue (`self.DamageType`))
  (bind _asbp_gun (cast `/Game/JCH/Blueprint/Items/Guns/BP_Gun` (`self.GetOwner`)))
  (`/Game/JCH/Blueprint/Items/Guns/BP_Gun.SpawnImpactFX` _asbp_gun HitLocation HitNormal (select `bool` (`KismetSystemLibrary.IsValid` _returnvalue_2) :`false` "/Game/JCH/PhysMats/Metal.Metal" :`true` (`MaterialInterface.GetPhysicalMaterial` _returnvalue_2)))
  (`self.K2_DestroyActor`))

(fn `UserConstructionScript`)