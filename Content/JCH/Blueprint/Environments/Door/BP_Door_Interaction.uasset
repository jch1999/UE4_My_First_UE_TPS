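; BP_Door_Interaction is an interactable door that swings open and closed when the player interacts with it.
; Entering or leaving interaction range toggles the mesh's custom depth rendering.
; Each interaction alternates through a FlipFlop between playing and reversing the DoorRotating timeline, which sets the mesh's yaw in world space, so the swing ignores the actor's placed rotation.
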(event `/Game/JCH/Blueprint/Items/BPI_Interaction.OnInteractionRangeEntered`
  (params (InPlayer :type "/Game/JCH/Blueprint/BP_Player_Character Object Reference"))
  (`PrimitiveComponent.SetRenderCustomDepth` (`self.StaticMesh`) true))

(event `/Game/JCH/Blueprint/Items/BPI_Interaction.OnInteractionRangeExited`
  (`PrimitiveComponent.SetRenderCustomDepth` (`self.StaticMesh`) false))

(event `/Game/JCH/Blueprint/Items/BPI_Interaction.OnInteracted`
  (params (InPlayer :type "/Game/JCH/Blueprint/BP_Player_Character Object Reference"))
  (`/Engine/EditorBlueprintResources/StandardMacros.FlipFlop`
    (:`A`
      (bind (_direction _rotation) (`Timeline|DoorRotating` :!label _label)
        (:`Update`
          (`SceneComponent.K2_SetWorldRotation` (`self.StaticMesh`) (`KismetMathLibrary.MakeRotator` 0.0 0.0 _rotation) false false))))
    (:`B`
      (goto _label :!via `Reverse`))))

(fn `UserConstructionScript`
  (`parent.UserConstructionScript`))