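; BP_Gun is an interactable hitscan firearm that players pick up or drop, toggling physics, collision and custom-depth highlighting.
; Fire consumes ammo, plays effects, sends diminishing recoil to its owner (reset by StopFire), then traces from camera and muzzle to apply point damage.
; Impact sound, decal and particles come from a physical-surface DataTable with a default fallback.
; Reload refills from reserve ammo, optionally accounting for dropped magazines.
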(event `self.ReceiveBeginPlay`
  (`self.SetWeaponState` (`self.WeaponState`))
  (`self.StopFire`)
  (set `self.LoadedAmmoCount` (`self.MagazineCapacity`)))

(event `/Game/JCH/Blueprint/Items/Guns/BPI_Weapon.Reload`
  ;[1 1 1] Weapon Reload
  (`self.Calculate Reload Ammo`))

(event `/Game/JCH/Blueprint/Items/BPI_Interaction.OnInteracted`
  (params (InPlayer :type "/Game/JCH/Blueprint/BP_Player_Character Object Reference"))
  (`/Game/JCH/Blueprint/BP_Player_Character.PickUp` InPlayer self)
  (`self.SetWeaponState` "NewEnumerator1"))

(event `/Game/JCH/Blueprint/Items/BPI_Interaction.OnInteractionRangeEntered`
  (params (InPlayer :type "/Game/JCH/Blueprint/BP_Player_Character Object Reference"))
  (`parent.OnInteractionRangeEntered` InPlayer)
  (`PrimitiveComponent.SetRenderCustomDepth` (`self.SkeletalMesh`) true))

(event `/Game/JCH/Blueprint/Items/BPI_Interaction.OnInteractionRangeExited`
  (`parent.OnInteractionRangeExited`)
  (`PrimitiveComponent.SetRenderCustomDepth` (`self.SkeletalMesh`) false))

(fn `Calculate Reload Ammo`
  (bind _ammocount (`self.AmmoCount`))
  (bind _returnvalue (`KismetMathLibrary.SelectInt` (`self.MagazineCapacity`) (- (`self.MagazineCapacity`) (`self.LoadedAmmoCount`)) (`self.bIsDropMagazine`)))
  ;[1 1 1] Weapon Reload
  (set `self.ReloadAmmoCount` (`KismetMathLibrary.SelectInt` _returnvalue _ammocount (> _ammocount _returnvalue)))
  (set `self.LoadedAmmoCount` (`KismetMathLibrary.SelectInt` (`self.MagazineCapacity`) (+ (`self.ReloadAmmoCount`) (`self.LoadedAmmoCount`)) (`self.bIsDropMagazine`)))
  (set `self.AmmoCount` (- (`self.AmmoCount`) (`self.ReloadAmmoCount`))))

(fn `Check Line Trace Hit`
  (params (PlayerCamera :type "CameraComponent Object Reference"))
  (returns (HitResult :type "HitResult Structure") (bIsResult :type Boolean))
  (bind _returnvalue (`SceneComponent.K2_GetComponentLocation` PlayerCamera))
  (bind _returnvalue_2 (`SceneComponent.GetSocketLocation` (`self.SkeletalMesh`) "MuzzleFlash"))
  (bind (_outhit _returnvalue_3) (`KismetSystemLibrary.LineTraceSingle` _returnvalue (+ _returnvalue (* (`SceneComponent.GetForwardVector` PlayerCamera) 12000.0)) "TraceTypeQuery1"))
  (bind (_bblockinghit _binitialoverlap _time _distance _location _impactpoint _normal _impactnormal _physmat _hitactor _hitcomponent _hitbonename _hititem _elementindex _faceindex _tracestart _traceend) (`GameplayStatics.BreakHitResult` _outhit))
  (bind (_outhit_2 _returnvalue_4) (`KismetSystemLibrary.LineTraceSingle` :`Start` _returnvalue_2 :`End` (+ _returnvalue_2 (* (`KismetMathLibrary.GetForwardVector` (`KismetMathLibrary.FindLookAtRotation` _returnvalue_2 (`KismetMathLibrary.SelectVector` _impactpoint _traceend _returnvalue_3))) 12000.0)) :`TraceChannel` "TraceTypeQuery3" :`DrawDebugType` "ForDuration"))
  (return _outhit_2 _returnvalue_4))

(fn `CheckLoadedAmmo`
  (returns (isLoadedAmmo :type Boolean))
  ;[1 1 1] Weapon Reload
  (if (> (`self.LoadedAmmoCount`) 0)
    (`/Engine/EditorBlueprintResources/StandardMacros.DecrementInt` (`self.LoadedAmmoCount`)
      (:`  `
        (return true)))
    (else
      (`GameplayStatics.PlaySoundAtLocation` (`self.EmptySound`) (`self.K2_GetActorLocation`) (struct) 10.0 1.0 0.0 null null null)
      (return false))))

(fn `Dropped`
  (`self.SetWeaponState` "NewEnumerator0"))

(fn `Fire`
  (params (PlayerCamera :type "CameraComponent Object Reference"))
  (bind _recoilinputyaw (`self.RecoilInputYaw`))
  (bind _recoilinputpitch (`self.RecoilInputPitch`))
  ;[1 1 1] Weapon Reload
  (bind _isloadedammo (`self.CheckLoadedAmmo`))
  (if _isloadedammo
    ;[1 1 1] WeaponFireEffect
    (`self.SpawnEffect` (`self.MuzzleFlashEffect`) (`self.MuzzleSocketName`) (0.0 0.0 0.0) (struct :`Yaw` 90.0))
    (`self.SpawnEffect` (`self.ShellEjectEffect`) (`self.ShellEjectSocketName`))
    (bind _firesound (`self.FireSound`)
      (:`then`
        (`GameplayStatics.PlaySoundAtLocation` _firesound (`self.K2_GetActorLocation`) (struct) 1.0 1.0 0.0 null null null))
      (:`else`
        _))
    ;[1 1 1] Fre Weapon
    ;;[1 1 1] Recoil
    (message `/Game/JCH/Blueprint/BPI_Character.AddRecoil` (`self.GetOwner`) (`self.RecoilRotation`) _recoilinputpitch _recoilinputyaw)
    (set `self.RecoilInputPitch` (* _recoilinputpitch 0.8))
    (set `self.RecoilInputYaw` (* _recoilinputyaw 0.8))
    ;;[1 1 1] Dynamic Spread Crosshair
    (bind (_hitresult _bisresult) (`self.Check Line Trace Hit` PlayerCamera))
    (bind (_bblockinghit _binitialoverlap _time _distance _location _impactpoint _normal _impactnormal _physmat _hitactor _hitcomponent _hitbonename _hititem _elementindex _faceindex _tracestart) (`GameplayStatics.BreakHitResult` _hitresult))
    ;[1 1 1] Hit By Bullets
    (`GameplayStatics.ApplyPointDamage` _hitactor 10.0 _tracestart _hitresult (`GameplayStatics.GetPlayerController` 0) self (`self.DamageType`))
    ;[1 1 1] BulletImpactEffects
    (if _bisresult
      (`self.SpawnImpactFX` _hitresult))))

(fn `GetAmmoCounts`
  (returns (AmmoCount :type Integer) (LoadedAmmoCount :type Integer))
  (return (`self.AmmoCount`) (`self.LoadedAmmoCount`)))

(fn `GetInteractionTextAtach`
  (returns (ParentComponent :type "SceneComponent Object Reference"))
  (return (`self.SkeletalMesh`)))

(fn `GetPhysicalSurfaceData`
  (params (PhysicalMaterial :type "PhysicalMaterial Object Reference"))
  (returns (PhysicalSurfaceData :type "/Game/JCH/Blueprint/PhysicalData/FPhyiscalSurfaceData Structure"))
  ;[1 1 1] 코멘트
  (bind _returnvalue (`|GetDataTableRow` "/Game/JCH/Blueprint/PhysicalData/DT_Pysical_Impact_FX.DT_Pysical_Impact_FX" (`|GetEnumeratorName` (`PhysicalMaterial.SurfaceType` PhysicalMaterial)))
    (:`then`
      (return _returnvalue))
    (:`RowNotFound`
      (bind _returnvalue_2 (`|GetDataTableRow` "/Game/JCH/Blueprint/PhysicalData/DT_Pysical_Impact_FX.DT_Pysical_Impact_FX" "SurfaceType_Default")
        (:`then`
          (return _returnvalue_2))
        (:`RowNotFound`
          (return))))))

(fn `GetWeaponTexture`
  (returns (WeaponTexture :type "Texture2D Object Reference"))
  (return (`self.WeaponTexture`)))

(fn `SetRecoilAccurency`
  (params (isRecoil :type Boolean))
  ;[1 1 1] Dynamic Crosshair
  (message `/Game/JCH/Blueprint/UserInterface/BPI_User_Interface.SetReticleAccurency` (`PlayerController.GetHUD` (`GameplayStatics.GetPlayerController` 0)) (`KismetMathLibrary.SelectFloat` 0.15 0.5 isRecoil)))

(fn `SetWeaponState`
  (params (NewState :type "/Game/JCH/Blueprint/Items/Guns/EWeaponState Enum" :default "NewEnumerator0"))
  (bind _skeletalmesh (`self.SkeletalMesh`))
  (bind _skeletalmesh_2 (`self.SkeletalMesh`))
  (bind _output_get (set `self.WeaponState` NewState))
  (switch `/Game/JCH/Blueprint/Items/Guns/EWeaponState` _output_get
    (:`NewEnumerator0`
      (`PrimitiveComponent.SetCollisionProfileName` (`self.Sphere`) "OverlapOnlyPawn" true)
      (`PrimitiveComponent.SetSimulatePhysics` _skeletalmesh true)
      (`PrimitiveComponent.SetCollisionProfileName` _skeletalmesh "DroppedWeaopn" true))
    (:`NewEnumerator1`
      (`PrimitiveComponent.SetCollisionProfileName` (`self.Sphere`) "NoCollision" true)
      (`PrimitiveComponent.SetSimulatePhysics` _skeletalmesh_2 false)
      (`PrimitiveComponent.SetCollisionProfileName` _skeletalmesh_2 "NoCollision" true)
      (`SceneComponent.ResetRelativeTransform` (`self.SkeletalMesh`)))))

(fn `SpawnEffect`
  (params (EffectTemplete :type "ParticleSystem Object Reference") (SocketName :type Name) (RelativeLocation :type "Vector Structure") (RelativeRotation :type "Rotator Structure"))
  (bind _skeletalmesh (`self.SkeletalMesh`))
  (bind (_returnvalue_roll _returnvalue_pitch _returnvalue_yaw) (`KismetMathLibrary.BreakRotator` (`SceneComponent.GetSocketRotation` _skeletalmesh "None")))
  (`/Engine/EditorBlueprintResources/StandardMacros.IsValid` EffectTemplete
    (:`Is Valid`
      (`GameplayStatics.SpawnEmitterAtLocation` EffectTemplete (+ RelativeLocation (`SceneComponent.GetSocketLocation` _skeletalmesh "None")) (`KismetMathLibrary.MakeRotator` (+ RelativeRotation_Roll _returnvalue_roll) (+ RelativeRotation_Pitch _returnvalue_pitch) (+ RelativeRotation_Yaw _returnvalue_yaw))))))

(fn `SpawnImpactFX`
  (params (HitResult :type "HitResult Structure"))
  (bind (_physicalsurfacedata_surface _physicalsurfacedata_impactparticlefx _physicalsurfacedata_impactsound_cue _physicalsurfacedata_impactdecal _physicalsurfacedata_decalsize) (break `/Game/JCH/Blueprint/PhysicalData/FPhyiscalSurfaceData` (`self.GetPhysicalSurfaceData` HitResult_PhysMat)))
  (`GameplayStatics.PlaySoundAtLocation` _physicalsurfacedata_impactsound_cue HitResult_ImpactPoint (struct) 1.0 1.0 0.0 null null null)
  (bind _returnvalue (`KismetMaterialLibrary.CreateDynamicMaterialInstance` _physicalsurfacedata_impactdecal))
  (`MaterialInstanceDynamic.SetScalarParameterValue` _returnvalue "Frame" (`KismetMathLibrary.Conv_IntToDouble` (`KismetMathLibrary.RandomIntegerInRange` 0 3)))
  (`GameplayStatics.SpawnDecalAtLocation` _returnvalue _physicalsurfacedata_decalsize HitResult_ImpactPoint (`self.MakeImpactDecalRotation` HitResult_ImpactNormal) (`self.ImpactDeaclLifeSpan`))
  (`GameplayStatics.SpawnEmitterAttached` _physicalsurfacedata_impactparticlefx null "None" HitResult_ImpactPoint (`self.MakeImpactParticleRotation` HitResult_ImpactNormal)))

(fn `StopFire`
  (set `self.RecoilInputPitch` (`self.RecoilInputPitchMax`))
  (set `self.RecoilInputYaw` (`self.RecoilInputYawMax`)))

(fn `UserConstructionScript`
  (`parent.UserConstructionScript`))