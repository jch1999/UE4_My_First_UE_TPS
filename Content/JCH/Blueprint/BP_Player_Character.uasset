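; Player character Blueprint for a shooter, handling movement, stances, aiming, two weapon slots and interaction.
; Crouch and aim move the camera between booms, while prone uses a timeline to resize the capsule, with a trace before standing.
; Weapons attach to mesh sockets, switching plays a montage, and firing requires aiming.
; Interface messages drive the anim instance, HUD reticle and overlapped interactables, while recoil kicks controller rotation.
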(event `self.ReceiveBeginPlay`
  (`parent.ReceiveBeginPlay`)
  ;[1 1 1] Aiming Pos Blend
  (set `self.ABP_Player_Character` (`SkeletalMeshComponent.GetAnimInstance` (`self.Mesh`))))

(event `InputAxis|Turn`
  (params (AxisValue :type "Float (single-precision)"))
  (`self.AddControllerYawInput` AxisValue))

(event `InputAxis|LookUp`
  (params (AxisValue :type "Float (single-precision)"))
  (`self.AddControllerPitchInput` AxisValue))

(event `InputAxis|MoveForward`
  (params (AxisValue :type "Float (single-precision)"))
  (bind (_returnvalue_roll _returnvalue_pitch _returnvalue_yaw) (`KismetMathLibrary.BreakRotator` (`self.GetControlRotation`)))
  ;[1 1 1] Movemnt Input
  (`self.AddMovementInput` (`KismetMathLibrary.GetForwardVector` (`KismetMathLibrary.MakeRotator` 0.0 0.0 _returnvalue_yaw)) AxisValue))

(event `InputAxis|MoveRight`
  (params (AxisValue :type "Float (single-precision)"))
  (bind (_returnvalue_roll _returnvalue_pitch _returnvalue_yaw) (`KismetMathLibrary.BreakRotator` (`self.GetControlRotation`)))
  ;[1 1 1] Movemnt Input
  (if (not (`self.bIsProne`))
    (`self.AddMovementInput` (`KismetMathLibrary.GetRightVector` (`KismetMathLibrary.MakeRotator` 0.0 0.0 _returnvalue_yaw)) AxisValue)))

(event `InputAction|Walk`
  (params (Key :type "Key Structure"))
  (bind _charactermovement (`self.CharacterMovement`))
  ;[1 1 1] Movement Mode
  (:`Pressed`
    (if (not (`self.bIsProne`))
      (set `CharacterMovementComponent.MaxWalkSpeed` (`self.WalkSpeed`) _charactermovement)))
  (:`Released`
    (if (not (`self.bIsProne`))
      (set `CharacterMovementComponent.MaxWalkSpeed` (`self.RunSpeed`) _charactermovement))))

(event `InputAction|Crouch`
  (params (Key :type "Key Structure"))
  (bind _charactermovement (`self.CharacterMovement`))
  ;[1 1 1] Crouch
  (:`Pressed`
    (if (`self.bIsProne`)
      (`self.ToggleProne`)
      (`KismetSystemLibrary.Delay` 1.3))
    (if (`self.bIsCrouched`)
      (`self.UnCrouch`)
      (set `CharacterMovementComponent.MaxWalkSpeedCrouched` (`self.RunSpeed`) _charactermovement)
      ;[1 1 1] Crouch Camera
      (`self.ChangeCameraBoom` false)
      (else
        (`self.Crouch`)
        (set `CharacterMovementComponent.MaxWalkSpeedCrouched` (`self.CrouchSpeed`) _charactermovement)
        (`self.ChangeCameraBoom` true)))))

(event `ToggleProne`
  (bind _returnvalue (`self.K2_GetActorLocation`))
  ;[1 1 1] Prone
  (set `self.StandHeight` (`KismetMathLibrary.SelectFloat` 60.0 88.0 (`self.bIsCrouched`)) :!label _label)
  (if (`self.bIsProne`)
    (bind (_outhit _returnvalue_2) (`KismetSystemLibrary.LineTraceSingle` _returnvalue (+ _returnvalue (* (`KismetMathLibrary.GetUpVector` (`self.K2_GetActorRotation`)) 180.0)) "TraceTypeQuery1"))
    (if (not _returnvalue_2)
      (set `self.bIsProne` false)
      (set `self.bGettingUp` true)
      (`|ExecutionSequence`
        (:`then_0`
          (`KismetSystemLibrary.Delay` 2.5)
          (set `CharacterMovementComponent.MaxWalkSpeed` (`self.RunSpeed`) (`self.CharacterMovement`)))
        (:`then_1`
          (bind (_direction _prone_track) (`Timeline|PronTransition` :!via `ReverseFromEnd` :!label _label_2)
            (:`Update`
              (`SceneComponent.K2_SetRelativeLocation` (`self.Mesh`) (`KismetMathLibrary.VLerp` (`KismetMathLibrary.MakeVector` 0.0 0.0 (* -1 (`self.StandHeight`))) (`KismetMathLibrary.MakeVector` 0.0 0.0 (`self.ProneZ`)) _prone_track) false false)
              (`CapsuleComponent.SetCapsuleSize` (`self.CapsuleComponent`) (`KismetMathLibrary.Lerp` (`self.StandRadius`) (`self.ProneSize`) _prone_track) (`KismetMathLibrary.Lerp` (`self.StandHeight`) (`self.ProneSize`) _prone_track) true))))))
    (else
      (set `self.bIsProne` true)
      (set `self.bGettingUp` false)
      (set `CharacterMovementComponent.MaxWalkSpeed` (`self.ProneSpeed`) (`self.CharacterMovement`))
      (goto _label_2))))

(event `InputAction|Prone`
  (params (Key :type "Key Structure"))
  ;[1 1 1] Prone
  (:`Pressed`
    (goto _label)))

(event `InputAction|ToggleAim`
  (params (Key :type "Key Structure"))
  (:`Pressed`
    (`self.AimDown` true)
    (`self.ChangeCameraBoom` (`self.bIsCrouched`) :!label _label))
  (:`Released`
    (`self.AimDown` false)
    (goto _label)))

(event `self.AimDown`
  (params (AimEnable :type Boolean))
  (bind _output_get (set `self.bIsAimDown` AimEnable))
  (set `self.bUseControllerRotationYaw` _output_get)
  (message `/Game/JCH/Blueprint/Animation/BPI_Character_Animation.EnableAim` (`self.ABP_Player_Character`) _output_get)
  (message `/Game/JCH/Blueprint/UserInterface/BPI_User_Interface.Enable_Reticle` (`PlayerController.GetHUD` (`GameplayStatics.GetPlayerController` 0)) _output_get))

(event `InputAction|SwitchWeapon`
  (params (Key :type "Key Structure"))
  ;[1 1 1] Switch Weapon
  (:`Pressed`
    (`self.CheckEquipedWeapon`
      (:`Is Valid`
        (`self.CheckUnequipedWeapon`
          (:`Is Valid`
            (`|PlayMontage` (`self.Mesh`) "/Game/JCH/Blueprint/Animation/AM_SwitchWeapon.AM_SwitchWeapon" 1.0 0.0 "StartSwitch")))))))

(event `InputAction|Fire`
  (params (Key :type "Key Structure"))
  ;[1 1 1] Fire Weapon
  (:`Pressed`
    (if (`self.bIsAimDown`)
      (bind _equipedwepon (`self.CheckEquipedWeapon`)
        (:`Is Valid`
          (`/Game/JCH/Blueprint/Items/Guns/BP_Gun.Fire` _equipedwepon (`self.Camera`)))))))

(event `self.AddRecoil`
  (params (RecoilRotation :type "Rotator Structure") (RecoilPitch :type "Float (single-precision)") (RecoilYaw :type "Float (single-precision)"))
  ;[1 1 1] Recoil
  (`self.SpreadCrosshair` RecoilPitch RecoilYaw)
  (message `/Game/JCH/Blueprint/Animation/BPI_Character_Animation.AddRecoil` (`self.ABP_Player_Character`) RecoilRotation))

(event `self.CapsuleComponent.OnComponentBeginOverlap`
  (params (OverlappedComponent :type "PrimitiveComponent Object Reference") (OtherActor :type "Actor Object Reference") (OtherComp :type "PrimitiveComponent Object Reference") (OtherBodyIndex :type Integer) (bFromSweep :type Boolean) (SweepResult :type "HitResult Structure (by ref)"))
  ;[1 1 1] Overlap
  (if (`KismetSystemLibrary.DoesImplementInterface` OtherActor "/Game/JCH/Blueprint/Items/BPI_Interaction.BPI_Interaction_C")
    (message `/Game/JCH/Blueprint/Items/BPI_Interaction.OnInteractionRangeEntered` OtherActor self)))

(event `self.CapsuleComponent.OnComponentEndOverlap`
  (params (OverlappedComponent :type "PrimitiveComponent Object Reference") (OtherActor :type "Actor Object Reference") (OtherComp :type "PrimitiveComponent Object Reference") (OtherBodyIndex :type Integer))
  ;[1 1 1] Overlap
  (if (`KismetSystemLibrary.DoesImplementInterface` OtherActor "/Game/JCH/Blueprint/Items/BPI_Interaction.BPI_Interaction_C")
    (message `/Game/JCH/Blueprint/Items/BPI_Interaction.OnInteractionRangeExited` OtherActor)))

(event `InputAction|Interaction`
  (params (Key :type "Key Structure"))
  (:`Pressed`
    (for _array_element (`PrimitiveComponent.GetOverlappingActors` (`self.CapsuleComponent`) "/Script/Engine.Actor")
      (if (`KismetSystemLibrary.DoesImplementInterface` _array_element "/Game/JCH/Blueprint/Items/BPI_Interaction.BPI_Interaction_C")
        (message `/Game/JCH/Blueprint/Items/BPI_Interaction.OnInteracted` _array_element self)))))

(fn `DropWeapon`
  (params (Weqapon :type "/Game/JCH/Blueprint/Items/Guns/BP_Gun Object Reference"))
  ;[1 1 1] Recoil
  (`self.SetOwner` Weqapon null)
  (`self.K2_DetachFromActor` Weqapon "KeepWorld" "KeepWorld" "KeepWorld")
  (`/Game/JCH/Blueprint/Items/Guns/BP_Gun.Dropped` Weqapon))

(fn `EquipWeapon`
  (params (Weapon :type "/Game/JCH/Blueprint/Items/Guns/BP_Gun Object Reference"))
  (`self.K2_AttachToComponent` Weapon (`self.Mesh`) "AssaultRifleHolster_Socket" "SnapToTarget" "SnapToTarget" "SnapToTarget" true))

(fn `GetWeaponSocket`
  (params (SocketName :type Name))
  (returns (SocketTransform :type "Transform Structure"))
  (bind _weapon (`self.Weapon`))
  (`/Engine/EditorBlueprintResources/StandardMacros.IsValid` _weapon
    (:`Is Valid`
      (return (`SceneComponent.GetSocketTransform` _weapon SocketName "RTS_World")))))

(fn `PickUp`
  (params (Weapon :type "/Game/JCH/Blueprint/Items/Guns/BP_Gun Object Reference"))
  (`self.PrimaryWeapon`
    (:`then`
      (`self.SecondaryWeapon`
        (:`then`
          (bind _equipedwepon (`self.CheckEquipedWeapon`)
            (:`Is Valid`
              (`self.DropWeapon` _equipedwepon)
              (`self.SetEquipedWeapon` null)
              (`self.PickUp` (`local.Weapon`)))))
        (:`else`
          (set `self.SecondaryWeapon` Weapon)
          ;[1 1 1] Recoil
          (`self.SetOwner` Weapon self :!label _label)
          (`|ExecutionSequence`
            (:`then_0`
              (bind _equipedwepon_2 (`self.CheckEquipedWeapon`)
                (:`Is Valid`
                  (`self.EquipWeapon` _equipedwepon_2))))
            (:`then_1`
              (bind _uneqipedweapon (`self.CheckUnequipedWeapon`)
                (:`Is Valid`
                  (`self.UnequipWeapon` _uneqipedweapon))))))))
    (:`else`
      (set `self.PrimaryWeapon` Weapon)
      (goto _label))))

(fn `SpreadCrosshair`
  (params (RecoilPitch :type "Float (double-precision)") (RecoilYaw :type "Float (double-precision)"))
  (bind _isrecoveryrecoil (message `/Game/JCH/Blueprint/Animation/BPI_Character_Animation.IsRecoveryRecoil` (`self.ABP_Player_Character`)))
  (if _isrecoveryrecoil
    (`self.AddControllerPitchInput` (`KismetMathLibrary.RandomFloatInRange` 0.0 RecoilPitch))
    (`self.AddControllerYawInput` (* (`KismetMathLibrary.RandomFloatInRange` 0.0 RecoilYaw) (`KismetMathLibrary.RandomFloatInRange` -1.0 1.0)))
    (else
      (bind _equipedwepon (`self.CheckEquipedWeapon`)
        (:`Is Valid`
          (`/Game/JCH/Blueprint/Items/Guns/BP_Gun.StopFire` _equipedwepon))))))

(fn `SwitchWeapon`
  (switch `/Game/JCH/Blueprint/EWeaponSlot` (`self.CurrentWeaponSlot`)
    (:`NewEnumerator0`
      (set `self.CurrentWeaponSlot` "NewEnumerator1"))
    (:`NewEnumerator1`
      (set `self.CurrentWeaponSlot` "NewEnumerator0")))
  (`|ExecutionSequence`
    (:`then_0`
      (bind _equipedwepon (`self.CheckEquipedWeapon`)
        (:`Is Valid`
          (`self.EquipWeapon` _equipedwepon))))
    (:`then_1`
      (bind _uneqipedweapon (`self.CheckUnequipedWeapon`)
        (:`Is Valid`
          (`self.UnequipWeapon` _uneqipedweapon))))))

(fn `UnequipWeapon`
  (params (Weapon :type "/Game/JCH/Blueprint/Items/Guns/BP_Gun Object Reference"))
  (`self.K2_AttachToComponent` Weapon (`self.Mesh`) "LuncherHolsterSocket" "SnapToTarget" "SnapToTarget" "SnapToTarget" true))

(fn `UserConstructionScript`
  (`parent.UserConstructionScript`))