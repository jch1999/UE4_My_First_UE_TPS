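; BP_Zombie is a zombie Blueprint with a melee attack and a simple health and death system.
; AttackTarget plays an attack montage and applies melee damage to the given actor on the OnAttack notify, so hits follow the animation.
; Incoming damage reduces Health, and reaching zero triggers a one-time death that disables capsule collision and ragdolls the mesh through physics simulation.
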(event `Attack Target`
  (params (OtherActor :type "Actor Object Reference"))
  (bind _notifyname (`|PlayMontage` (`self.Mesh`) "/Game/JCH/Blueprint/AI/newAnim/AM_ZombieAttack.AM_ZombieAttack")
    (:`OnNotifyBegin`
      (if (== _notifyname "OnAttack")
        (`GameplayStatics.ApplyDamage` OtherActor 10.0 (`self.GetController`) self "/Game/JCH/Blueprint/Items/Guns/DamageTypes/BP_Zombie_MeleeDamageType.BP_Zombie_MeleeDamageType_C")))))

(event `self.ReceiveAnyDamage`
  (params (Damage :type "Float (single-precision)") (DamageType :type "DamageType Object Reference") (InstigatedBy :type "Controller Object Reference") (DamageCauser :type "Actor Object Reference"))
  (if (> (`self.Health`) 0)
    (bind _output_get (set `self.Health` (- (`self.Health`) (`KismetMathLibrary.FTrunc` Damage))))
    (if (not (> _output_get 0))
      (`/Engine/EditorBlueprintResources/StandardMacros.DoOnce` false
        (:`Completed`
          (`PrimitiveComponent.SetCollisionEnabled` (`self.CapsuleComponent`) "NoCollision")
          (`PrimitiveComponent.SetSimulatePhysics` (`self.Mesh`) true))))))

(fn `UserConstructionScript`)